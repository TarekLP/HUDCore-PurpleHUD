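; HUDCore mod actor that lets custom HUD mods replace or sit alongside the vanilla action-phase HUD.
; On BeginPlay it scans the asset registry for HUD data assets and loads them as PDA_CustomHUD default objects.
; It builds saved settings categories from that data and adds each HUD widget to the action-phase overlay.
; Visibility toggles drive render opacity on custom and vanilla HUDs, updating when settings change.
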(event Custom|RefreshHUDs
  ;[0 0 0] Hides vanilla HUD and shows custom HUD
  (CallFunction|PrinttoModLoader "Refreshing HUD")
  (Utilities|FlowControl|Delay 1.0)
  (CallFunction|GetActionPhaseWidgets)
  (for _array_element (Variables|Default|GetSM_ActionPhase_Base)
    (EventDispatchers|BindEventtoOnSettingsChanged (Variables|/Game/UI/Widgets/StateMachine/ActionPhase/WBP_UI_SM_ActionPhaseMenu.WBP_UI_SM_ActionPhaseMenu_C|GetWidget_Settings_HUDCore (Variables|/Game/UI/Widgets/StateMachine/WBP_UI_SM_ActionPhase.WBP_UI_SM_ActionPhase_C|GetWidget_PauseMenu _array_element)) (EventDispatchers|CreateEvent :!event Custom|OnSettingsChanged))
    (if (Widget|IsVisible _array_element) :!label _label
      (bind _arrayelement (Utilities|Array|ReverseforEachLoop (Variables|Default|GetUnparsedHUDData))
        (:LoopBody
          (Utilities|FlowControl|Sequence
            (:then_0
              (if (Utilities|IsValidClass (Variables|/Game/Mods/_NadzMods/HUDCore/PDA_CustomHUD.PDA_CustomHUD_C|GetMainWidget _arrayelement))
                (bind _exists (CallFunction|DoesHUDAlreadyExist _array_element (Variables|/Game/Mods/_NadzMods/HUDCore/PDA_CustomHUD.PDA_CustomHUD_C|GetMainWidget _arrayelement)))
                (if _exists
                  (bind _returnvalue (CallFunction|GetVanillaHUDOpacity))
                  (Widget|SetRenderOpacity (Variables|/Game/UI/Widgets/StateMachine/WBP_UI_SM_ActionPhase.WBP_UI_SM_ActionPhase_C|GetVanillaHUD_Panel _array_element) _returnvalue)
                  (else
                    (bind _returnvalue_2 (UserInterface|CreateWidget (Variables|/Game/Mods/_NadzMods/HUDCore/PDA_CustomHUD.PDA_CustomHUD_C|GetMainWidget _arrayelement) (Class|SBZPlayerLibrary|GetLocalPlayerController)))
                    (CallFunction|PrinttoModLoader (Utilities|String|ToString(Text) (Utilities|Text|FormatText "Attempting to create {Class}: 
Spawned {W}" (Utilities|GetClassDisplayName (Variables|/Game/Mods/_NadzMods/HUDCore/PDA_CustomHUD.PDA_CustomHUD_C|GetMainWidget _arrayelement)) (Utilities|GetDisplayName _returnvalue_2))))
                    (bind _returnvalue_3 (CallFunction|GetVanillaHUDOpacity))
                    (Widget|SetRenderOpacity (Variables|/Game/UI/Widgets/StateMachine/WBP_UI_SM_ActionPhase.WBP_UI_SM_ActionPhase_C|GetVanillaHUD_Panel _array_element) _returnvalue_3)
                    (bind _returnvalue_4 (Widget|Panel|AddChild (Variables|/Game/UI/Widgets/StateMachine/WBP_UI_SM_ActionPhase.WBP_UI_SM_ActionPhase_C|GetOverlay_HUDs _array_element) _returnvalue_2))
                    (bind _asoverlay_slot (Utilities|Casting|CastToOverlaySlot _returnvalue_4))
                    (Layout|GridSlot|SetHorizontalAlignment _asoverlay_slot "HAlign_Fill")
                    (Layout|GridSlot|SetVerticalAlignment _asoverlay_slot "VAlign_Fill")
                    (Default|AddNavigationButton (Variables|/Game/UI/Widgets/StateMachine/ActionPhase/WBP_UI_SM_ActionPhaseMenu.WBP_UI_SM_ActionPhaseMenu_C|GetWidget_Settings_HUDCore (Variables|/Game/UI/Widgets/StateMachine/WBP_UI_SM_ActionPhase.WBP_UI_SM_ActionPhase_C|GetWidget_PauseMenu _array_element)) (Utilities|Text|ToText(Name) (Variables|/Game/Mods/_NadzMods/HUDCore/PDA_CustomHUD.PDA_CustomHUD_C|GetUniqueID _arrayelement)))
                    (Default|CreateButtons (Variables|/Game/Mods/_NadzMods/HUDCore/Settings/WBP_Settings_Screen_Category_HUDCore.WBP_Settings_Screen_Category_HUDCore_C|GetModsettingsButtonNavbar (Variables|/Game/UI/Widgets/StateMachine/ActionPhase/WBP_UI_SM_ActionPhaseMenu.WBP_UI_SM_ActionPhaseMenu_C|GetWidget_Settings_HUDCore (Variables|/Game/UI/Widgets/StateMachine/WBP_UI_SM_ActionPhase.WBP_UI_SM_ActionPhase_C|GetWidget_PauseMenu _array_element))))
                    (Default|BindButtonClicks (Variables|/Game/Mods/_NadzMods/HUDCore/Settings/WBP_Settings_Screen_Category_HUDCore.WBP_Settings_Screen_Category_HUDCore_C|GetModsettingsButtonNavbar (Variables|/Game/UI/Widgets/StateMachine/ActionPhase/WBP_UI_SM_ActionPhaseMenu.WBP_UI_SM_ActionPhaseMenu_C|GetWidget_Settings_HUDCore (Variables|/Game/UI/Widgets/StateMachine/WBP_UI_SM_ActionPhase.WBP_UI_SM_ActionPhase_C|GetWidget_PauseMenu _array_element))))
                    (Utilities|Array|Add (Variables|/Game/UI/Widgets/StateMachine/WBP_UI_SM_ActionPhase.WBP_UI_SM_ActionPhase_C|GetCustomHUDs _array_element) _returnvalue_2)))
                (else
                  (CallFunction|PrinttoModLoader (Utilities|String|ToString(Text) (Utilities|Text|FormatText " {Class} is not valid!!!" (Utilities|GetClassDisplayName (Variables|/Game/Mods/_NadzMods/HUDCore/PDA_CustomHUD.PDA_CustomHUD_C|GetMainWidget _arrayelement))))))))
            (:then_1
              (for _array_element_2 (Variables|/Game/UI/Widgets/StateMachine/WBP_UI_SM_ActionPhase.WBP_UI_SM_ActionPhase_C|GetCustomHUDs _array_element)
                (if (== (Variables|/Game/Mods/_NadzMods/HUDCore/PDA_CustomHUD.PDA_CustomHUD_C|GetMainWidget _arrayelement) (Utilities|GetClass _array_element_2))
                  (bind _returnvalue_5 (CallFunction|GetCustomHUDOpacity (Variables|/Game/Mods/_NadzMods/HUDCore/PDA_CustomHUD.PDA_CustomHUD_C|GetUniqueID _arrayelement)))
                  (Widget|SetRenderOpacity _array_element_2 _returnvalue_5)))))))
      (else
        (Utilities|FlowControl|Delay 0.2)
        (goto _label)))))

(event Custom|OnEndPlayEvent
  (params (Actor :type Actor%20Object%20Reference) (EndPlayReason :type EEndPlayReason%20Enum :default "Destroyed"))
  (bind _sm_actionphase_base (Variables|Default|GetSM_ActionPhase_Base))
  ;[0 0 0] Hides vanilla HUD and shows custom HUD
  (for _array_element _sm_actionphase_base
    (Widget|RemovefromParent _array_element)
    (Utilities|Platform|CollectGarbage))
  (Utilities|Array|Clear _sm_actionphase_base))

(event Custom|InitializeHUDs
  (CallFunction|PrinttoModLoader "Initializing HUDs")
  (Utilities|FlowControl|Delay 0.5)
  (Utilities|FlowControl|Sequence
    (:then_0
      (CallFunction|GetActionPhaseWidgets))
    (:then_1
      (CallFunction|CreateHUDSettings))
    (:then_2
      (CallFunction|RefreshHUDs))))

(event Custom|GetActionPhaseWidgets
  ;[0 0 0] Gets reference to vanilla action phase main widget and parent widget that custom HUDs should be added to
  (bind _foundwidgets (Widget|GetAllWidgetsOfClass "/Game/UI/Widgets/StateMachine/WBP_UI_SM_ActionPhase.WBP_UI_SM_ActionPhase_C" false :!label _label))
  (if (> (Utilities|Array|Length _foundwidgets) 0)
    (for _array_element _foundwidgets
      (Utilities|Array|AddUnique (Variables|Default|GetSM_ActionPhase_Base) _array_element))
    (else
      (Utilities|FlowControl|Delay 1.0)
      (goto _label))))

(event Custom|ResetCategory
  (params (ModName :type Name))
  (bind _categoryname (CallFunction|GetCategoryNamefromModName ModName))
  (bind _config (CallFunction|LoadConfig (Utilities|String|ToString(Name) _categoryname)))
  (Utilities|Map|Clear (Variables|/Game/Mods/_NadzMods/HUDCore/Settings/SaveGame_HUDCore_Settings.SaveGame_HUDCore_Settings_C|GetToggleMap _config))
  (Utilities|Map|Clear (Variables|/Game/Mods/_NadzMods/HUDCore/Settings/SaveGame_HUDCore_Settings.SaveGame_HUDCore_Settings_C|GetFloatMap _config))
  (Utilities|Map|Clear (Variables|/Game/Mods/_NadzMods/HUDCore/Settings/SaveGame_HUDCore_Settings.SaveGame_HUDCore_Settings_C|GetColorMap _config))
  (CallFunction|SaveConfig _config (Utilities|String|ToString(Name) _categoryname)))

(event Custom|OnSettingsChanged
  ;[0 0 0] Hides vanilla HUD and shows custom HUD
  (Default|CallSettingsChanged)
  (for _array_element (Variables|Default|GetSM_ActionPhase_Base)
    (Utilities|FlowControl|Sequence
      (:then_0
        (for _array_element_2 (Variables|Default|GetUnparsedHUDData)
          (for _array_element_3 (Variables|/Game/UI/Widgets/StateMachine/WBP_UI_SM_ActionPhase.WBP_UI_SM_ActionPhase_C|GetCustomHUDs _array_element)
            (if (== (Variables|/Game/Mods/_NadzMods/HUDCore/PDA_CustomHUD.PDA_CustomHUD_C|GetMainWidget _array_element_2) (Utilities|GetClass _array_element_3))
              (bind _returnvalue (CallFunction|GetCustomHUDOpacity (Variables|/Game/Mods/_NadzMods/HUDCore/PDA_CustomHUD.PDA_CustomHUD_C|GetUniqueID _array_element_2)))
              (bind _value (CallFunction|GetShouldShowHUDs "General"))
              (Widget|SetRenderOpacity _array_element_3 (Math|Float|SelectFloat _returnvalue 0.0 _value)))))
        (bind _returnvalue_2 (CallFunction|GetVanillaHUDOpacity))
        (Widget|SetRenderOpacity (Variables|/Game/UI/Widgets/StateMachine/WBP_UI_SM_ActionPhase.WBP_UI_SM_ActionPhase_C|GetVanillaHUD_Panel _array_element) _returnvalue_2)))))

(event EventBeginPlay
  (bind _filter (Variables|Default|GetFilter))
  (|CallParentFunction)
  (bind _returnvalue (Class|SBZEventLibrary|GetGameEventBroker))
  (EventDispatchers|BindEventtoOnActionPhaseEntered _returnvalue (EventDispatchers|CreateEvent :!event Custom|InitializeHUDs))
  (Game|BindEventtoOnEndPlay (EventDispatchers|CreateEvent :!event Custom|OnEndPlayEvent))
  ;[0 0 0] Finds custom HUD data assets and initialises them
  (Class|AssetRegistry|ScanPathsSynchronous (Class|AssetRegistryHelpers|GetAssetRegistry) (Utilities|Array|MakeArray "/Game/Mods/HUDs/Data") true)
  (bind _outassetdata (Class|AssetRegistry|GetAssets (Class|AssetRegistryHelpers|GetAssetRegistry) (Utilities|MakeARFilter 0 (.packagepaths _filter) 0 (.classnames _filter) 0 (.brecursivepaths _filter) (.brecursiveclasses _filter))))
  (bind _output_get (Variables|Default|SetOut%20Asset%20Data _outassetdata))
  (for _array_element _output_get
    (CallFunction|PrinttoModLoader (Utilities|String|ToString(Text) (Utilities|Text|FormatText "Found {DA} with a class of {C}" (Utilities|String|Replace (Class|KismetSystemLibrary|GetPathName (Class|AssetRegistryHelpers|GetAsset _array_element)) "." ".Default__") (Utilities|GetClassDisplayName (Utilities|GetClass (Class|AssetRegistryHelpers|GetAsset _array_element))))))
    (bind _returnvalue_2 (Utilities|LoadAssetBlocking (Class|KismetSystemLibrary|ToSoftObjRef(SoftObjPath) (Utilities|MakeSoftObjectPath (Utilities|String|Replace (Class|KismetSystemLibrary|GetPathName (Class|AssetRegistryHelpers|GetAsset _array_element)) "." ".Default__")))))
    (bind _aspda_custom_hud (Utilities|Casting|CastToPDA_CustomHUD _returnvalue_2))
    (Utilities|Array|AddUnique (Variables|Default|GetUnparsedHUDData) _aspda_custom_hud)))

(fn ConstructionScript
  (|CallParentFunction))

(fn ParseHUDData
  (params (DA :type PDA%20Custom%20HUD%20Object%20Reference)))

(fn CreateHUDSettings
  (Utilities|FlowControl|Sequence
    (:then_0
      (CallFunction|CreateGeneralCategory))
    (:then_1
      (for _array_element (Variables|Default|GetUnparsedHUDData)
        (Utilities|Array|Clear (LocalVariables|GetGroups))
        (bind _categoryname (CallFunction|GetCategoryNamefromModName (Variables|/Game/Mods/_NadzMods/HUDCore/PDA_CustomHUD.PDA_CustomHUD_C|GetUniqueID _array_element)))
        (bind (_config _firsttime) (CallFunction|LoadConfig (Utilities|String|ToString(Name) _categoryname)))
        (for _array_element_2 (Variables|/Game/Mods/_NadzMods/HUDCore/PDA_CustomHUD.PDA_CustomHUD_C|GetGroups _array_element)
          (Utilities|Array|Clear (LocalVariables|GetCurrentSettings))
          (Utilities|FlowControl|Sequence
            (:then_0
              (for _array_element_3 (.ToggleSettings (Utilities|Struct|BreakFHUDCore_Settings_Group _array_element_2))
                (bind _sbzsettingdata (CallFunction|CreateToggleSetting (.UniqueID (Utilities|Struct|BreakFHUDCore_Settings_Bool _array_element_3)) (Utilities|Text|ToText(String) (.DisplayText (Utilities|Struct|BreakFHUDCore_Settings_Bool _array_element_3))) true "None" "None" "None" (select (or (not (.ReturnValue (Utilities|Map|Find (Variables|/Game/Mods/_NadzMods/HUDCore/Settings/SaveGame_HUDCore_Settings.SaveGame_HUDCore_Settings_C|GetToggleMap _config) (.UniqueID (Utilities|Struct|BreakFHUDCore_Settings_Bool _array_element_3))))) _firsttime) (.DefaultValue (Utilities|Struct|BreakFHUDCore_Settings_Bool _array_element_3)) (.Value (Utilities|Map|Find (Variables|/Game/Mods/_NadzMods/HUDCore/Settings/SaveGame_HUDCore_Settings.SaveGame_HUDCore_Settings_C|GetToggleMap _config) (.UniqueID (Utilities|Struct|BreakFHUDCore_Settings_Bool _array_element_3)))))))
                (Utilities|Array|Add (LocalVariables|GetCurrentSettings) _sbzsettingdata)))
            (:then_1
              (for _array_element_4 (.FloatSettings (Utilities|Struct|BreakFHUDCore_Settings_Group _array_element_2))
                (bind _sbzsettingdata_2 (CallFunction|CreateFloatSetting (.UniqueID (Utilities|Struct|BreakFHUDCore_Settings_Float _array_element_4)) (Utilities|Text|ToText(String) (.DisplayText (Utilities|Struct|BreakFHUDCore_Settings_Float _array_element_4))) true "None" "None" "None" (.Min (Utilities|Struct|BreakFHUDCore_Settings_Float _array_element_4)) (.Max (Utilities|Struct|BreakFHUDCore_Settings_Float _array_element_4)) (.IncrementValue (Utilities|Struct|BreakFHUDCore_Settings_Float _array_element_4)) (Math|Float|SelectFloat (.DefaultValue (Utilities|Struct|BreakFHUDCore_Settings_Float _array_element_4)) (.Value (Utilities|Map|Find (Variables|/Game/Mods/_NadzMods/HUDCore/Settings/SaveGame_HUDCore_Settings.SaveGame_HUDCore_Settings_C|GetFloatMap _config) (.UniqueID (Utilities|Struct|BreakFHUDCore_Settings_Float _array_element_4)))) (or (not (.ReturnValue (Utilities|Map|Find (Variables|/Game/Mods/_NadzMods/HUDCore/Settings/SaveGame_HUDCore_Settings.SaveGame_HUDCore_Settings_C|GetFloatMap _config) (.UniqueID (Utilities|Struct|BreakFHUDCore_Settings_Float _array_element_4))))) _firsttime))))
                (Utilities|Array|Add (LocalVariables|GetCurrentSettings) _sbzsettingdata_2)))
            (:then_2
              (for _array_element_5 (.ColorSettings (Utilities|Struct|BreakFHUDCore_Settings_Group _array_element_2))
                (bind _sbzsettingdata_3 (CallFunction|CreateColorSetting (.UniqueID (Utilities|Struct|BreakFHUDCore_Settings_Color _array_element_5)) (Utilities|Text|ToText(String) (.DisplayText (Utilities|Struct|BreakFHUDCore_Settings_Color _array_element_5))) true "None" "None" "None" (Math|Color|SelectColor (.DefaultValue (Utilities|Struct|BreakFHUDCore_Settings_Color _array_element_5)) (.Value (Utilities|Map|Find (Variables|/Game/Mods/_NadzMods/HUDCore/Settings/SaveGame_HUDCore_Settings.SaveGame_HUDCore_Settings_C|GetColorMap _config) (.UniqueID (Utilities|Struct|BreakFHUDCore_Settings_Color _array_element_5)))) (or (not (.ReturnValue (Utilities|Map|Find (Variables|/Game/Mods/_NadzMods/HUDCore/Settings/SaveGame_HUDCore_Settings.SaveGame_HUDCore_Settings_C|GetColorMap _config) (.UniqueID (Utilities|Struct|BreakFHUDCore_Settings_Color _array_element_5))))) _firsttime))))
                (Utilities|Array|Add (LocalVariables|GetCurrentSettings) _sbzsettingdata_3)))
            (:then_3
              (bind _array (CallFunction|CreateSettingsGroup (Variables|/Game/Mods/_NadzMods/HUDCore/PDA_CustomHUD.PDA_CustomHUD_C|GetUniqueID _array_element) (.UniqueID (Utilities|Struct|BreakFHUDCore_Settings_Group _array_element_2)) (Utilities|String|StringToName (.DisplayText (Utilities|Struct|BreakFHUDCore_Settings_Group _array_element_2))) (LocalVariables|GetCurrentSettings)))
              (Utilities|Array|AppendArray (LocalVariables|GetGroups) _array))))
        (CallFunction|CreateSettingCategory (Variables|/Game/Mods/_NadzMods/HUDCore/PDA_CustomHUD.PDA_CustomHUD_C|GetUniqueID _array_element) (LocalVariables|GetGroups))
        (CallFunction|SaveConfig _config (Utilities|String|ToString(Name) _categoryname))))))

(fn CreateGeneralCategory
  (bind _returnvalue (Utilities|Name|MakeLiteralName "HUDCore_General_bShouldShowVanlillaHUD"))
  (bind _returnvalue_2 (Utilities|Name|MakeLiteralName "HUDCore_General_bShouldShowCustomHUD"))
  (bind _categoryname (CallFunction|GetCategoryNamefromModName "General" :!label _label))
  (bind _config (CallFunction|LoadConfig (Utilities|String|ToString(Name) _categoryname)))
  (bind _keys (Utilities|Map|Keys (Variables|/Game/Mods/_NadzMods/HUDCore/Settings/SaveGame_HUDCore_Settings.SaveGame_HUDCore_Settings_C|GetToggleMap _config)))
  (if (> (Utilities|Array|Length _keys) 0)
    (LocalVariables|SetCurrentBools _keys)
    (Utilities|FlowControl|Sequence
      (:then_0
        (for (_array_element _array_index) (Variables|Default|GetUnparsedHUDData)
          (bind _categoryname_2 (CallFunction|GetCategoryNamefromModName "General"))
          (bind (_value _successful) (CallFunction|GetToggleSettingValue (Utilities|String|ToString(Name) _categoryname_2) (Utilities|String|StringToName (Utilities|String|ToString(Text) (Utilities|Text|FormatText "HUDCore_General_bShouldShow{ID}" (Variables|/Game/Mods/_NadzMods/HUDCore/PDA_CustomHUD.PDA_CustomHUD_C|GetUniqueID _array_element))))))
          (CallFunction|SetToggleSettingValue (Utilities|String|ToString(Name) _categoryname) (Utilities|String|StringToName (Utilities|String|ToString(Text) (Utilities|Text|FormatText "HUDCore_General_bShouldShow{ID}" (Variables|/Game/Mods/_NadzMods/HUDCore/PDA_CustomHUD.PDA_CustomHUD_C|GetUniqueID _array_element)))) (select _successful _value (== _array_index 0))))
        (bind _config_2 (CallFunction|LoadConfig (Utilities|String|ToString(Name) _categoryname)))
        (bind _keys_2 (Utilities|Map|Keys (Variables|/Game/Mods/_NadzMods/HUDCore/Settings/SaveGame_HUDCore_Settings.SaveGame_HUDCore_Settings_C|GetToggleMap _config_2)))
        (LocalVariables|SetCurrentBools _keys_2))
      (:then_1
        (if (Utilities|Array|ContainsItem (LocalVariables|GetCurrentBools) "HUDCore_General_bShouldShowCustomHUD")
          (bind _sbzsettingdata (CallFunction|CreateToggleSetting _returnvalue_2 (Utilities|Text|ToText(Name) "Enable Custom HUDs") true "None" "None" "None" (.Value (Utilities|Map|Find (Variables|/Game/Mods/_NadzMods/HUDCore/Settings/SaveGame_HUDCore_Settings.SaveGame_HUDCore_Settings_C|GetToggleMap _config) _returnvalue_2))))
          (Utilities|Array|Add (LocalVariables|GetSettings) _sbzsettingdata)
          (Utilities|Array|RemoveItem (LocalVariables|GetCurrentBools) "HUDCore_General_bShouldShowCustomHUD")
          (if (Utilities|Array|ContainsItem (LocalVariables|GetCurrentBools) "HUDCore_General_bShouldShowVanlillaHUD")
            (bind _sbzsettingdata_2 (CallFunction|CreateToggleSetting _returnvalue (Utilities|Text|ToText(Name) "Enable Vanilla HUD") true "None" "None" "None" (.Value (Utilities|Map|Find (Variables|/Game/Mods/_NadzMods/HUDCore/Settings/SaveGame_HUDCore_Settings.SaveGame_HUDCore_Settings_C|GetToggleMap _config) _returnvalue))))
            (Utilities|Array|Add (LocalVariables|GetSettings) _sbzsettingdata_2)
            (Utilities|Array|RemoveItem (LocalVariables|GetCurrentBools) "HUDCore_General_bShouldShowVanlillaHUD")
            (for _array_element_2 (LocalVariables|GetCurrentBools)
              (for _array_element_3 (Variables|Default|GetUnparsedHUDData)
                (if (Utilities|Name|Equal(Name) _array_element_2 (Utilities|String|StringToName (Utilities|String|ToString(Text) (Utilities|Text|FormatText "HUDCore_General_bShouldShow{ID}" (Variables|/Game/Mods/_NadzMods/HUDCore/PDA_CustomHUD.PDA_CustomHUD_C|GetUniqueID _array_element_3)))))
                  (bind _value_2 (CallFunction|GetToggleSettingValue (Utilities|String|ToString(Name) _categoryname) _array_element_2))
                  (bind _sbzsettingdata_3 (CallFunction|CreateToggleSetting _array_element_2 (Utilities|Text|ToText(Name) (Variables|/Game/Mods/_NadzMods/HUDCore/PDA_CustomHUD.PDA_CustomHUD_C|GetDisplayName _array_element_3)) true "None" "None" "None" _value_2))
                  (Utilities|Array|Add (LocalVariables|GetSettings) _sbzsettingdata_3))))
            (bind _array (CallFunction|CreateSettingsGroup "General" "General" "General" (LocalVariables|GetSettings)))
            (CallFunction|CreateSettingCategory "General" _array)))))
    (else
      (CallFunction|SetToggleSettingValue (Utilities|String|ToString(Name) _categoryname) (Utilities|Name|MakeLiteralName "HUDCore_General_bShouldShowCustomHUD") (Class|KismetSystemLibrary|MakeLiteralBool true))
      (CallFunction|SetToggleSettingValue (Utilities|String|ToString(Name) _categoryname) (Utilities|Name|MakeLiteralName "HUDCore_General_bShouldShowVanlillaHUD") (Class|KismetSystemLibrary|MakeLiteralBool false))
      (goto _label))))

(fn DoesHUDAlreadyExist
  (params (Target :type WBP%20UI%20SM%20Action%20Phase%20Object%20Reference) (HUDClass :type Object%20Class%20Reference))
  (bind _array_element (Utilities|Array|ForEachLoopwithBreak (Variables|/Game/UI/Widgets/StateMachine/WBP_UI_SM_ActionPhase.WBP_UI_SM_ActionPhase_C|GetCustomHUDs Target) :!label _label)
    (:LoopBody
      (if (== (Utilities|GetClass _array_element) HUDClass)
        (LocalVariables|SetFound true)
        (CallFunction|PrinttoModLoader (Utilities|String|ToString(Text) (Utilities|Text|FormatText "{HUD} already exists " (Utilities|GetClassDisplayName HUDClass))))
        (goto _label Break)
        (else
          (LocalVariables|SetFound false))))
    (:Completed
      (return (LocalVariables|GetFound)))))

(fn GetVanillaHUDOpacity
  (bind _categoryname (CallFunction|GetCategoryNamefromModName "General"))
  (bind _value (CallFunction|GetToggleSettingValue (Utilities|String|ToString(Name) _categoryname) (Utilities|Name|MakeLiteralName "HUDCore_General_bShouldShowVanlillaHUD")))
  (return (Math|Float|SelectFloat 1.0 0.0 _value)))

(fn GetCustomHUDOpacity
  (params (ModName :type Name))
  (bind _categoryname (CallFunction|GetCategoryNamefromModName "General"))
  (bind _value (CallFunction|GetToggleSettingValue (Utilities|String|ToString(Name) _categoryname) (Utilities|String|StringToName (Utilities|String|ToString(Text) (Utilities|Text|FormatText "HUDCore_General_bShouldShow{ID}" ModName)))))
  (return (Math|Float|SelectFloat 1.0 0.0 _value)))

(fn GetShouldShowHUDs
  (params (ModName :type Name))
  (bind _categoryname (CallFunction|GetCategoryNamefromModName ModName))
  (bind _value (CallFunction|GetToggleSettingValue (Utilities|String|ToString(Name) _categoryname) (Utilities|String|StringToName (Utilities|String|ToString(Text) (Utilities|Text|FormatText "HUDCore_General_bShouldShowCustomHUD")))))
  (return _value))